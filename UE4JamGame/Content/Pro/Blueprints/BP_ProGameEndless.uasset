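; BP_ProGameEndless procedurally generates an endless side-view platforming course along X.
; BeginPlay derives jump limits from the player's movement and gravity, then starts FireNextPlatform, which re-fires every half second.
; Each pass randomizes width and gap, caps height using the jump arc, and spawns BP_Platform, sometimes with BP_Monster.
; CheatMode grants invincibility and a player-following floor; origin shifting and an older spawner are disconnected.
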(event Custom|FireNextPlatform
  (bind _returnvalue (Game|GetPlayerCharacter 0))
  (bind _platformmingap (Variables|Default|GetPlatformMinGap))
  (bind _maxjumpdistance (Variables|Default|GetMaxJumpDistance))
  (bind _platformxthreshold (Variables|Default|GetPlatformXThreshold))
  (bind _platformzthreshold (Variables|Default|GetPlatformZThreshold))
  (bind _returnvalue_2 (Math|Random|RandomFloatinRange _platformmingap _maxjumpdistance))
  (bind _charactermovement (Variables|/Script/Engine.Character|GetCharacterMovement _returnvalue))
  ;[1 1 1] Calculate next Spawn
  ;;[0 1 0] Width
  (Variables|Default|SetPreviousPlatformWidth (Variables|Default|GetCurrentPlatformWidth))
  (bind _output_get (Variables|Default|SetCurrentPlatformWidth (Math|Random|RandomFloatinRange (Variables|Default|GetPlatformMinWidth) (Variables|Default|GetPlatformMaxWidth))))
  ;;[1 0 0] Position
  (bind _output_get_2 (Variables|Default|SetCurrentPlatformGap (select (> _returnvalue_2 _platformxthreshold) (- _returnvalue_2 _platformxthreshold) _returnvalue_2)))
  (Variables|Default|SetPreviousPlatformSpawnPositionX (Variables|Default|GetCurrentPlatformSpawnPositionX))
  (bind _output_get_3 (Variables|Default|SetCurrentPlatformSpawnPositionX (+ (Variables|Default|GetCurrentPlatformSpawnPositionX) (Variables|Default|GetPreviousPlatformWidth) _output_get_2)))
  ;;[0 0 1] Height
  (Variables|Default|SetPreviousPlatformSpawnPositionZ (Variables|Default|GetCurrentPlatformSpawnPositionZ))
  (bind _output_get_4 (Variables|Default|SetCurrentPlatformSpawnPositionZ (select (> (Math|Random|RandomFloatinRange (Variables|Default|GetPlatformMinHeight) (|(h+((Vy*t)-((0.500000*g)*(t*t)))) (Variables|/Script/Engine.CharacterMovementComponent|GetJumpZVelocity _charactermovement) (Variables|Default|GetGravityPositive) (|(x/Vx) (Variables|Default|GetCurrentPlatformGap) (Variables|/Script/Engine.CharacterMovementComponent|GetMaxWalkSpeed _charactermovement)) (Variables|Default|GetCurrentPlatformSpawnPositionZ))) _platformzthreshold) (- (Math|Random|RandomFloatinRange (Variables|Default|GetPlatformMinHeight) (|(h+((Vy*t)-((0.500000*g)*(t*t)))) (Variables|/Script/Engine.CharacterMovementComponent|GetJumpZVelocity _charactermovement) (Variables|Default|GetGravityPositive) (|(x/Vx) (Variables|Default|GetCurrentPlatformGap) (Variables|/Script/Engine.CharacterMovementComponent|GetMaxWalkSpeed _charactermovement)) (Variables|Default|GetCurrentPlatformSpawnPositionZ))) _platformzthreshold) (Math|Random|RandomFloatinRange (Variables|Default|GetPlatformMinHeight) (|(h+((Vy*t)-((0.500000*g)*(t*t)))) (Variables|/Script/Engine.CharacterMovementComponent|GetJumpZVelocity _charactermovement) (Variables|Default|GetGravityPositive) (|(x/Vx) (Variables|Default|GetCurrentPlatformGap) (Variables|/Script/Engine.CharacterMovementComponent|GetMaxWalkSpeed _charactermovement)) (Variables|Default|GetCurrentPlatformSpawnPositionZ))))))
  (Game|SpawnActorfromClass "/Game/Pro/Blueprints/BP_Platform.BP_Platform_C" (Math|Transform|MakeTransform (Math|Vector|MakeVector _output_get_3 0.0 _output_get_4) "0.000000, 0, 0" "1.000000,1,1") "Undefined" 0 (select (> (Variables|Default|GetCurrentPlatformSpawnPositionZ) (+ (Variables|Default|GetPreviousPlatformSpawnPositionZ) (Variables|Default|GetSoftPlatformMinHeightThreshold))) "NewEnumerator1" "NewEnumerator0") "0.0,0.0,0.0" (Math|Vector|MakeVector _output_get 0.0 0.0) true true false)
  (if (> (Math|Random|RandomFloat) (Variables|Default|GetPlatformMobSpawnChance))
    _
    (else
      (Game|SpawnActorfromClass "/Game/Pro/Blueprints/BP_Monster.BP_Monster_C" (Math|Transform|MakeTransform (Math|Vector|MakeVector (+ (Variables|Default|GetCurrentPlatformSpawnPositionX) (/ (Variables|Default|GetCurrentPlatformWidth) 2.0)) 0.0 (+ (Variables|Default|GetCurrentPlatformSpawnPositionZ) 2e+01)) "0, 0, 0" "1,1,1") "Undefined" 0 (select (> (Math|Random|RandomFloat) 0.5) "1.000000,0,0" "-1.000000,0,0") 0)))
  (Development|PrintString "New Platform Spawned!")
  (Utilities|FlowControl|Delay 0.5)
  (CallFunction|FireNextPlatform))

(event EventBeginPlay
  (bind _returnvalue (Game|GetPlayerCharacter 0))
  (bind _charactermovement (Variables|/Script/Engine.Character|GetCharacterMovement _returnvalue))
  (bind _returnvalue_2 (Components|Movement|GetGravityZ _charactermovement))
  (bind _jumpzvelocity (Variables|/Script/Engine.CharacterMovementComponent|GetJumpZVelocity _charactermovement))
  ;[1 1 1] Calculate Jump Distance and Height
  (Variables|Default|SetGravityPositive (Math|Float|Absolute(Float) _returnvalue_2))
  (Variables|Default|SetMaxJumpDistance (* (* (|((2*v)/g) _jumpzvelocity _returnvalue_2) -1.0) (Variables|/Script/Engine.CharacterMovementComponent|GetMaxWalkSpeed _charactermovement)))
  (Variables|Default|SetMaxJumpHeight (* (|((v*v)/(2*g)) _jumpzvelocity _returnvalue_2) -1.0))
  (bind _asbp_pro_player (Utilities|Casting|CastToBP_ProPlayer _returnvalue)
    (:then
      (Variables|/Game/Pro/Blueprints/BP_ProPlayer.BP_ProPlayer_C|SetInvincible _asbp_pro_player (Variables|Default|GetCheatMode)))
    (:CastFailed
      _))
  (CallFunction|FireNextPlatform)
  (if (Variables|Default|GetCheatMode)
    (bind _returnvalue_3 (Game|SpawnActorfromClass "/Game/Pro/Blueprints/BP_Platform.BP_Platform_C" (Math|Transform|MakeTransform (Math|Vector|MakeVector 0.0 0.0 (+ (Variables|Default|GetPlatformMinHeight) -5e+01)) "0.000000, 0, 0" "1.000000,1,1") "Undefined" 0 "NewEnumerator0" "0.0,0.0,0.000000" (Math|Vector|MakeVector 2e+02 0.0 0.0) true true false))))

(event EventTick
  (params (DeltaSeconds :type Float%20%28single-precision%29))
  (Utilities|FlowControl|Sequence
    (:then_0
      (if (Variables|Default|GetCheatMode)
        (Transformation|SetActorLocation (stale EventBeginPlay _returnvalue_3) (Math|Vector|MakeVector (- (.x (Transformation|GetActorLocation (Game|GetPlayerCharacter 0))) 1e+02) (.y (Transformation|GetActorLocation (stale EventBeginPlay _returnvalue_3))) (.z (Transformation|GetActorLocation (stale EventBeginPlay _returnvalue_3)))) false false)))))

(fn ConstructionScript)