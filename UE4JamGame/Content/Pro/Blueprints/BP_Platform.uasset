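; Paper2D platform actor, Solid or Soft, built from a row of left, middle and right sprite segments.
; The construction script tiles sprites between two rounded widget points at fixed spacing, then fits the trigger and collision box to that span.
; While BP_ProPlayer overlaps DownTrigger, Soft platforms ignore a collision channel, restoring blocking on exit.
; Collision uses either individual segments or one box, with optional projectile blocking.
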(event OnComponentBeginOverlap(DownTrigger)
  (params (OverlappedComponent :type Primitive%20Component%20Object%20Reference) (OtherActor :type Actor%20Object%20Reference) (OtherComp :type Primitive%20Component%20Object%20Reference) (OtherBodyIndex :type Integer) (bFromSweep :type Boolean) (SweepResult :type Hit%20Result%20Structure%20%28by%20ref%29))
  (Utilities|Casting|CastToBP_ProPlayer OtherActor
    (:then
      (switch Utilities|FlowControl|Switch|SwitchonPlatformType (Variables|Default|GetPlatformType)
        (:NewEnumerator1
          (if (Variables|Default|GetIndividiualSegmentCollision)
            (for _array_element (Variables|Default|GetPlatform%20Parts%20Array)
              (Collision|SetCollisionResponsetoChannel _array_element "ECC_GameTraceChannel2" "ECR_Ignore"))
            (else
              (Collision|SetCollisionResponsetoChannel (Variables|Default|GetCollision) "ECC_GameTraceChannel2" "ECR_Ignore"))))))
    (:CastFailed
      (Development|PrintString (Utilities|String|Append "WARNING " (Utilities|GetObjectName OtherActor)) true true "(R=1.000000,G=0.098612,B=0.390662,A=1.000000)"))))

(event OnComponentEndOverlap(DownTrigger)
  (params (OverlappedComponent :type Primitive%20Component%20Object%20Reference) (OtherActor :type Actor%20Object%20Reference) (OtherComp :type Primitive%20Component%20Object%20Reference) (OtherBodyIndex :type Integer))
  (Utilities|Casting|CastToBP_ProPlayer OtherActor)
  (switch Utilities|FlowControl|Switch|SwitchonPlatformType (Variables|Default|GetPlatformType)
    (:NewEnumerator1
      (if (Variables|Default|GetIndividiualSegmentCollision)
        (for _array_element (Variables|Default|GetPlatform%20Parts%20Array)
          (Collision|SetCollisionResponsetoChannel _array_element "ECC_GameTraceChannel2" "ECR_Block"))
        (else
          (Collision|SetCollisionResponsetoChannel (Variables|Default|GetCollision) "ECC_GameTraceChannel2" "ECR_Block"))))))

(fn ConstructionScript
  (bind _collision (Variables|Default|GetCollision))
  (bind _platform_parts_array (Variables|Default|GetPlatform%20Parts%20Array))
  (bind _triggeroffset (Variables|Default|GetTriggerOffset))
  (bind _triggerscale (Variables|Default|GetTriggerScale))
  (bind _triggerextrasize (Variables|Default|GetTriggerExtraSize))
  (bind _output (Utilities|Array|Get(acopy) _platform_parts_array))
  (bind _boxextent (Collision|GetComponentBounds _output))
  (Variables|Default|SetRoundedLeftWidget (CallFunction|RoundVector (Variables|Default|GetPlatform%20Left%20Widget)))
  (Variables|Default|SetRoundedRightWidget (CallFunction|RoundVector (Variables|Default|GetPlatform%20Right%20Widget)))
  (Utilities|FlowControl|Sequence
    (:then_0
      (Components|Box|SetBoxExtent (Variables|Default|GetDownTrigger) (Math|Vector|MakeVector (+ (* (/ (- (.x (Variables|Default|GetRoundedRightWidget)) (.x (Variables|Default|GetRoundedLeftWidget))) 2.0) (.x _triggerscale)) (.x _triggerextrasize)) (+ (.y _triggerextrasize) (.y _triggerscale)) (+ (.z _triggerextrasize) (.z _triggerscale))) true)
      (Transformation|SetRelativeLocation (Variables|Default|GetDownTrigger) (Math|Vector|MakeVector (+ (/ (+ (.x (Variables|Default|GetRoundedRightWidget)) (.x (Variables|Default|GetRoundedLeftWidget))) 2.0) (.x _triggeroffset)) (.y _triggeroffset) (Utilities|CalculateTriggerZOffset (.z _triggeroffset) (Variables|Default|GetAutoOffsetTriggerZ))) false false)
      (Collision|SetCollisionEnabled (Variables|Default|GetDownTrigger) (Utilities|Select :Index (Variables|Default|GetPlatformType) :NewEnumerator0 "QueryAndPhysics" :NewEnumerator1 "QueryAndPhysics")))
    (:then_1
      (for _index (range 0 (- (Math|Float|Floor (/ (- (.x (Variables|Default|GetRoundedRightWidget)) (.x (Variables|Default|GetRoundedLeftWidget))) (Variables|Default|GetSpacing))) 1))
        (bind _index_2 (Utilities|CompareIndexMacro _index 0 (- (Math|Float|Floor (/ (- (.x (Variables|Default|GetRoundedRightWidget)) (.x (Variables|Default|GetRoundedLeftWidget))) (Variables|Default|GetSpacing))) 1))
          (:Left
            (CallFunction|AddNewPart _index_2 (Variables|Default|GetLeftSprite)))
          (:Right
            (CallFunction|AddNewPart _index_2 (Variables|Default|GetRightSprite)))
          (:Mid
            (CallFunction|AddNewPart _index_2 (Variables|Default|GetMidSprite)))))
      (CallFunction|SetIndividualSegmentCollision (Variables|Default|GetIndividiualSegmentCollision)))
    (:then_2
      (Components|Box|SetBoxExtent (Variables|Default|GetCollision) (Math|Vector|MakeVector (/ (- (.x (Variables|Default|GetRoundedRightWidget)) (.x (Variables|Default|GetRoundedLeftWidget))) 2.0) (.y _boxextent) (.z _boxextent)) true)
      (Transformation|SetRelativeLocation _collision (Math|Vector|MakeVector (/ (+ (.x (Variables|Default|GetRoundedRightWidget)) (.x (Variables|Default|GetRoundedLeftWidget))) 2.0) 0.0 0.0) false false)
      (Collision|SetCollisionResponsetoChannel _collision "ECC_GameTraceChannel1" (select (Variables|Default|GetBlockProjectiles) "ECR_Block" "ECR_Ignore")))))

(fn AddNewPart
  (params (Index :type Integer) (Sprite :type Paper%20Sprite%20Object%20Reference))
  (bind _spacing (Variables|Default|GetSpacing))
  (bind _returnvalue (AddComponent|AddPaperSpriteComponent false (Math|Transform|MakeTransform (Math|Vector|MakeVector (+ (+ (* Index _spacing) (/ _spacing 2.0)) (.x (Variables|Default|GetRoundedLeftWidget))) 0.0 0.0) "0.000000, 0, 0" "1,1,1")))
  (Utilities|Array|Add (Variables|Default|GetPlatform%20Parts%20Array) _returnvalue)
  (Rendering|Components|Sprite|SetSprite _returnvalue Sprite)
  (Collision|SetCollisionEnabled _returnvalue "QueryAndPhysics")
  (Collision|SetCollisionObjectType _returnvalue "ECC_GameTraceChannel4")
  (Collision|SetCollisionResponsetoChannel _returnvalue "ECC_GameTraceChannel4" "ECR_Ignore")
  (Collision|SetCollisionResponsetoChannel _returnvalue "ECC_GameTraceChannel1" (select (Variables|Default|GetBlockProjectiles) "ECR_Block" "ECR_Ignore")))

(fn RoundVector
  (params (Vector :type Vector))
  (return (Math|Vector|MakeVector (Math|Conversions|ToFloat(Integer) (Math|Float|Round (.x Vector))) (Math|Conversions|ToFloat(Integer) (Math|Float|Round (.y Vector))) (Math|Conversions|ToFloat(Integer) (Math|Float|Round (.z Vector))))))

(fn SetBlockProjectiles
  (params (BlockProjectiles :type Boolean))
  (Variables|Default|SetBlockProjectiles BlockProjectiles)
  (for _array_element (Variables|Default|GetPlatform%20Parts%20Array)
    (Collision|SetCollisionResponsetoChannel _array_element "ECC_GameTraceChannel1" (select BlockProjectiles "ECR_Block" "ECR_Ignore"))))

(fn SetIndividualSegmentCollision
  (params (Collision :type Boolean))
  (Variables|Default|SetIndividiualSegmentCollision Collision)
  (for _array_element (Variables|Default|GetPlatform%20Parts%20Array)
    (Collision|SetCollisionEnabled _array_element (select Collision "QueryAndPhysics" "NoCollision")))
  (Collision|SetCollisionEnabled (Variables|Default|GetCollision) (select Collision "NoCollision" "QueryAndPhysics")))