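; Patrolling enemy pawn that walks back and forth on a platform and damages BP_Player on sprite overlap or capsule hit.
; Each Tick a downward trace assigns the BP_Platform beneath it, and FrontCollision is compared with that platform's edge points to reverse movement and facing.
; The construction script toggles blocking on a custom collision channel via CollideWithFriendly.
; AnyDamage is empty; health and score logic is disconnected, and control rotation is marked not working.
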(event OnComponentHit(CapsuleComponent)
  (params (HitComponent :type Primitive%20Component%20Object%20Reference) (OtherActor :type Actor%20Object%20Reference) (OtherComp :type Primitive%20Component%20Object%20Reference) (NormalImpulse :type Vector :default "0, 0, 0") (Hit :type Hit%20Result%20Structure%20%28by%20ref%29))
  (bind _asbp_player (Utilities|Casting|CastToBP_Player OtherActor))
  (Game|Damage|ApplyDamage _asbp_player 25.0 (Pawn|GetController) self))

(event OnComponentHit(Sprite)
  (params (HitComponent :type Primitive%20Component%20Object%20Reference) (OtherActor :type Actor%20Object%20Reference) (OtherComp :type Primitive%20Component%20Object%20Reference) (NormalImpulse :type Vector :default "0, 0, 0") (Hit :type Hit%20Result%20Structure%20%28by%20ref%29)))

(event OnComponentBeginOverlap(Sprite)
  (params (OverlappedComponent :type Primitive%20Component%20Object%20Reference) (OtherActor :type Actor%20Object%20Reference) (OtherComp :type Primitive%20Component%20Object%20Reference) (OtherBodyIndex :type Integer) (bFromSweep :type Boolean) (SweepResult :type Hit%20Result%20Structure%20%28by%20ref%29))
  (bind _asbp_player (Utilities|Casting|CastToBP_Player OtherActor))
  (Game|Damage|ApplyDamage _asbp_player 25.0 (Pawn|GetController) self))

(event EventBeginPlay
  ;[1 1 1] Initial movement
  (Pawn|Input|AddMovementInput (Variables|Default|GetInitialDirection) 1.0 false))

(event Collision|EventActorBeginOverlap
  (params (OtherActor :type Actor%20Object%20Reference)))

(event EventTick
  (params (DeltaSeconds :type Float%20%28single-precision%29))
  (bind _returnvalue (Transformation|GetActorLocation))
  (bind _returnvalue_2 (Class|Pawn|GetLastMovementInputVector))
  (bind _frontcollision (Variables|Default|GetFrontCollision))
  (bind _returnvalue_3 (Transformation|GetWorldLocation _frontcollision))
  ;[1 1 1] Assign Platform and Movement
  (bind _outhit (Collision|LineTraceForObjects (Math|Vector|MakeVector (.x _returnvalue) (.y _returnvalue) (.z _returnvalue)) (Math|Vector|MakeVector (.x _returnvalue) (.y _returnvalue) (* (Variables|Default|GetMaxLineTraceDistance) -1.0)) (Utilities|Array|MakeArray "ObjectTypeQuery2" "ObjectTypeQuery10") false 0 "ForOneFrame")) ; TODO: Do front linetrace to check for colliding objects, not just vertical linetrace
  (bind _asbp_platform (Utilities|Casting|CastToBP_Platform (.hitactor _outhit))
    (:then
      (if (== _asbp_platform (Variables|Default|GetAssignedPlatform))
        _
        (else
          (Development|PrintString "New Platform assigned!")))
      (bind _output_get (Variables|Default|SetAssignedPlatform _asbp_platform))
      (Pawn|Input|AddMovementInput (select (select (Variables|Default|GetOrientation) (< (.x (- _returnvalue_3 (Math|Transform|TransformLocation (Transformation|GetActorTransform _output_get) (Variables|/Game/Game/Blueprints/BP_Platform.BP_Platform_C|GetPlatform%20Right%20Widget _output_get)))) 0.0) (> (.x (- _returnvalue_3 (Math|Transform|TransformLocation (Transformation|GetActorTransform _output_get) (Variables|/Game/Game/Blueprints/BP_Platform.BP_Platform_C|GetPlatform%20Left%20Widget _output_get)))) 0.0)) _returnvalue_2 (* _returnvalue_2 -1.0)) 1.0 false)
      (Math|Float|CompareFloat (.X (Math|Vector|BreakVector (select (select (Variables|Default|GetOrientation) (< (.x (- _returnvalue_3 (Math|Transform|TransformLocation (Transformation|GetActorTransform _output_get) (Variables|/Game/Game/Blueprints/BP_Platform.BP_Platform_C|GetPlatform%20Right%20Widget _output_get)))) 0.0) (> (.x (- _returnvalue_3 (Math|Transform|TransformLocation (Transformation|GetActorTransform _output_get) (Variables|/Game/Game/Blueprints/BP_Platform.BP_Platform_C|GetPlatform%20Left%20Widget _output_get)))) 0.0)) _returnvalue_2 (* _returnvalue_2 -1.0)))) 0.0
        (:>
          (Variables|Default|SetOrientation true :!label _label)
          (Pawn|SetControlRotation (Pawn|GetController) (Math|Rotator|MakeRotator 0.0 0.0 0.0)) ; Not working
          (Transformation|SetActorRotation "0, 0, 0"))
        (:==
          (Pawn|Input|AddMovementInput (Variables|Default|GetInitialDirection) 1.0 false)
          (goto _label))
        (:<
          (Variables|Default|SetOrientation false)
          (Pawn|SetControlRotation (Pawn|GetController) (Math|Rotator|MakeRotator 0.0 0.0 1.8e+02)) ; Not working
          (Transformation|SetActorRotation "0,180.000000, 0"))))
    (:CastFailed
      (Development|PrintString (Utilities|String|Append "WARNING AI " (Utilities|GetObjectName self) " HAS NO PLATFORM ASSIGNED") true true "(R=1.000000,G=0.000000,B=0.000000,A=1.000000)"))))

(event Game|Damage|EventAnyDamage
  (params (Damage :type Float%20%28single-precision%29) (DamageType :type Damage%20Type%20Object%20Reference) (InstigatedBy :type Controller%20Object%20Reference) (DamageCauser :type Actor%20Object%20Reference))
  ;[1 1 1] Damage Actor
)

(fn ConstructionScript
  (if (Variables|Default|GetCollideWithFriendly)
    (Collision|SetCollisionResponsetoChannel (Variables|Collision|GetCapsuleComponent) "ECC_GameTraceChannel3" "ECR_Block")
    (Collision|SetCollisionResponsetoChannel (Variables|Default|GetSprite) "ECC_GameTraceChannel3" "ECR_Block")
    (else
      (Collision|SetCollisionResponsetoChannel (Variables|Collision|GetCapsuleComponent) "ECC_GameTraceChannel3" "ECR_Ignore")
      (Collision|SetCollisionResponsetoChannel (Variables|Default|GetSprite) "ECC_GameTraceChannel3" "ECR_Ignore"))))