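; BP_Background is a background plane actor that follows the player along the X axis.
; Every tick it copies the X location of player 0's controlled pawn, keeping its own Y and Z.
; The construction script applies the MeshScale and BackgroundMaterial variables to the EditorPlane component and sets its fixed world rotation.
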(event EventTick
  (params (DeltaSeconds :type Float%20%28single-precision%29))
  (bind _returnvalue (Transformation|GetActorLocation))
  (Transformation|SetActorLocation (Math|Vector|MakeVector (.x (Transformation|GetActorLocation (Pawn|GetControlledPawn (Game|GetPlayerController 0)))) (.y _returnvalue) (.z _returnvalue)) false false))

(fn ConstructionScript
  (bind _editorplane (Variables|Default|GetEditorPlane))
  (Transformation|SetWorldScale3D _editorplane (Variables|Default|GetMeshScale))
  (Rendering|Material|SetMaterial _editorplane 0 (Variables|Default|GetBackgroundMaterial))
  (Transformation|SetWorldRotation _editorplane "0,-90.000000, 0" false false))