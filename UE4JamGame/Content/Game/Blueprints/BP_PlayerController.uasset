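; Player controller Blueprint that puts the HUD on screen and holds score-adding logic.
; BeginPlay creates the BP_HUD widget, stores it and adds it to the viewport.
; AddScore applies a sum to Score, clamping negative results to zero unless CanBeNegative is set.
; A ScoreChanged event prints the change, old and new scores for debugging, though AddScore does not call it.
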(event Custom|ScoreChanged
  (params (ScoreChange :type Integer) (OldScore :type Integer) (NewScore :type Integer))
  (Development|PrintString (Utilities|String|Append "Score has changed: " (Utilities|String|ToString(Integer) ScoreChange) " Old Score: " (Utilities|String|ToString(Integer) OldScore) " New Score: " (Utilities|String|ToString(Integer) NewScore)) true true "(R=0.996819,G=0.000000,B=1.000000,A=1.000000)"))

(event EventTick
  (params (DeltaSeconds :type Float%20%28single-precision%29)))

(event EventBeginPlay
  (bind _returnvalue (UserInterface|CreateWidget "/Game/Game/UI/BP_HUD.BP_HUD_C"))
  (bind _output_get (Variables|Default|SetHUD _returnvalue))
  (UserInterface|Viewport|AddtoViewport _output_get 0))

(fn ConstructionScript)

(fn AddScore
  (params (Score :type Integer) (CanBeNegative :type Boolean))
  (if (>= (+ Score (Variables|Default|GetScore)) 0) ; Checks if score is negative
    (Variables|Default|SetScore (+ Score (Variables|Default|GetScore)) :!label _label)
    (elif CanBeNegative ; Checks if score can be negative
      (goto _label)
      (else
        (Variables|Default|SetScore 0)))))